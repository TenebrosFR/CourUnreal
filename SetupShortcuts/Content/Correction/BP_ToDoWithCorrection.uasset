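; Training Blueprint, apparently an exercise to-do with its correction, with French instructions for learning Blueprint editor basics.
; The 00_Shortcuts graph drills aligning nodes, recreating Branch, MultiGate, Sequence and Delay nodes with shortcuts, and adding variables.
; The 01_Variables graph covers Print String output and demonstrates disabled nodes within execution chains.
; Its custom events have no callers here, and the default events and Construction Script are empty.
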(event EventBeginPlay)

(event Collision|EventActorBeginOverlap
  (params (OtherActor :type Actor%20Object%20Reference)))

(event EventTick
  (params (DeltaSeconds :type Float%20%28single-precision%29)))

(event Custom|Ex0
  ;[0 1 0.5261] 01 Commencer ici
  ;;[0 1 0.5261] Alligner les nodes suivant
  (Utilities|FlowControl|MultiGate false false -1
    (:Out%200
      (if true
        _))))

(event Custom|Print%20values
  ;[0 1 0.5261] Commencer Ici
  ;;[0 1 0.5261] Faire afficher dans la console de log et à l’écran la valeur de plusieurs variables
  ;; Vous utiliserez le node Print String
  (Development|PrintString "Hello"))

(event Custom|TestDisableNode
  ;[0 1 0.5261] Commencer Ici
  ;;[0 1 0.5261] Démontrer les disable / enable et dev only sur les nodes ( F6, F7 et F8 )
  (Development|PrintString "Avant Node" true true "(R=1.000000,G=0.024355,B=0.000000,A=1.000000)" 1e+01)
  (Development|PrintString "Disable")
  (Development|PrintString "Après " true true "(R=0.000000,G=0.660000,B=1.000000,A=1.000000)" 1e+01)
  (Utilities|FlowControl|Sequence
    (:then_0
      (if false
        (Development|PrintString "Vrai" true true "(R=0.000000,G=0.660000,B=1.000000,A=1.000000)" 1e+01)
        (else
          (Development|PrintString "False" true true "(R=0.000000,G=0.660000,B=1.000000,A=1.000000)" 1e+01))))
    (:then_1
      (Development|PrintString "Hello" true true "(R=0.000000,G=0.660000,B=1.000000,A=1.000000)" 1e+01))))

(fn ConstructionScript)